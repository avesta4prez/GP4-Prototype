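; Blueprint that switches the level between two sets of static mesh objects, World A and World B, so only one is active at a time.
; ToggleWorlds flips WorldAIsActive and passes each array to SetWorldVisibility with opposite states.
; SetWorldVisibility toggles both mesh visibility and collision, so hidden objects stop blocking.
; BeginPlay runs one toggle, so play starts in the opposite of the flag's initial state.
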(event `Toggle Worlds`
  (bind _worlda (`self.WorldA`))
  (bind _worldb (`self.WorldB`))
  (if (`self.WorldA_IsActive`)
    (`self.Set World Visibility` _worlda)
    (`self.Set World Visibility` _worldb true)
    (set `self.WorldA_IsActive` false)
    (else
      (`self.Set World Visibility` _worlda true)
      (`self.Set World Visibility` _worldb)
      (set `self.WorldA_IsActive` true))))

(event `Set World Visibility`
  (params (WorldArray :type "Array of StaticMeshActor Object Reference") (Visible :type Boolean))
  (for _array_element WorldArray
    (bind _staticmeshcomponent (`StaticMeshActor.StaticMeshComponent` _array_element))
    (`SceneComponent.SetVisibility` _staticmeshcomponent Visible true)
    (if Visible
      (`PrimitiveComponent.SetCollisionEnabled` _staticmeshcomponent "QueryAndPhysics")
      (else
        (`PrimitiveComponent.SetCollisionEnabled` _staticmeshcomponent "NoCollision")))))

(event `self.ReceiveBeginPlay`
  (`self.Toggle Worlds`))

(fn `UserConstructionScript`)